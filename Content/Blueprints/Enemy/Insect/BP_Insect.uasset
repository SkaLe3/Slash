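; Insect enemy Blueprint that adds reactive buzzing audio and a physics-driven death to its parent class.
; Timelines modulate the Buzz pitch and volume on attack, non-fatal hit and death, stopping the sound when the death curve finishes.
; On death the mesh switches to physics simulation with an upward kick.
; Sufficiently hard mesh impacts then play a ground-hit sound and trigger a landing surface-impact effect.
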(event `self.ReceiveTick`
  (params (DeltaSeconds :type "Float (single-precision)"))
  (`parent.ReceiveTick` DeltaSeconds))

(event `AttackStart`
  (bind _buzz (`self.Buzz`))
  (bind (_direction _pitch _volume) (`Timeline|AttackPitchVolume` :!via `PlayFromStart`)
    (:`Update`
      (`AudioComponent.SetPitchMultiplier` _buzz (* (`self.BasePitch`) _pitch))
      (`AudioComponent.SetVolumeMultiplier` _buzz (* (`self.BaseVolume`) _volume)))))

(event `self.Die`
  (bind _mesh (`self.Mesh`))
  (bind _buzz (`self.Buzz`))
  ; Change pitch and volume on die
  (`parent.Die`)
  (`PrimitiveComponent.SetCollisionEnabled` _mesh "QueryAndPhysics")
  (`PrimitiveComponent.SetSimulatePhysics` _mesh true)
  (`PrimitiveComponent.AddImpulse` (`self.Mesh`) (0.0 0.0 1000.0) "None" true)
  (`PrimitiveComponent.SetNotifyRigidBodyCollision` (`self.Mesh`) true)
  (bind (_direction _newtrack_1 _newtrack_0) (`Timeline|DiePitchVolume`)
    (:`Update`
      (`AudioComponent.SetPitchMultiplier` _buzz (* (`self.BasePitch`) _newtrack_1))
      (`AudioComponent.SetVolumeMultiplier` _buzz (* (`self.BaseVolume`) _newtrack_0)))
    (:`Finished`
      (`AudioComponent.Stop` _buzz))))

(event `self.Mesh.OnComponentHit`
  (params (HitComponent :type "PrimitiveComponent Object Reference") (OtherActor :type "Actor Object Reference") (OtherComp :type "PrimitiveComponent Object Reference") (NormalImpulse :type "Vector Structure") (Hit :type "HitResult Structure (by ref)"))
  ; Body hit ground sound
  (if (>= (`KismetMathLibrary.VSize` NormalImpulse) 10000.0)
    (`GameplayStatics.PlaySoundAtLocation` "/Game/Assets/Audio/MetaSounds/sfx_GroundHitLight.sfx_GroundHitLight" Hit_ImpactPoint (struct) 1.0 1.0 0.0 null null null null)
    (`self.OnCharacterSurfaceImpact` "None" "EIT_Land" (make `SurfaceImpactEventData` Hit_ImpactPoint 2.5 1.0 1.0 false false false true))))

(event `HitInterface.GetHit`
  (params (ImpactPoint :type "Vector Structure (by ref)") (Hitter :type "Actor Object Reference"))
  ; Change pitch and volume on hit
  (`parent.GetHit` ImpactPoint Hitter)
  (if (not (`self.IsDead`))
    (bind (_direction _newtrack_1 _newtrack_2) (`Timeline|HitPitchVolume` :!via `PlayFromStart`)
      (:`Update`
        (`AudioComponent.SetPitchMultiplier` (`self.Buzz`) _newtrack_1)
        (`AudioComponent.SetVolumeMultiplier` (`self.Buzz`) _newtrack_2)))))

(fn `UserConstructionScript`
  (`parent.UserConstructionScript`))