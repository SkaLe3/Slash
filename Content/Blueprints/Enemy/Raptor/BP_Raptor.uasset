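; Raptor enemy Blueprint whose own logic is a death dissolve, with Tick deferring to the parent class.
; DissolveBody scales the FadeOut timeline's play rate by the inverse of DeathLifeSpan, then writes its value to the FadeOut scalar parameter on every material in DissolveMaterials.
; BeginPlay and overlap events are disabled, and leftover debug-sphere draws for three radii are never executed.
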(event `self.ReceiveTick`
  (params (DeltaSeconds :type "Float (single-precision)"))
  (`parent.ReceiveTick` DeltaSeconds))

(event `self.Dissolve Body`
  (`TimelineComponent.SetPlayRate` (`self.FadeOut`) (/ 1.0 (`self.DeathLifeSpan`)))
  (bind (_direction _newtrack_0) (`Timeline|FadeOut`)
    (:`Update`
      (for _array_element (`self.DissolveMaterials`)
        (`MaterialInstanceDynamic.SetScalarParameterValue` _array_element "FadeOut" _newtrack_0)))))

(fn `UserConstructionScript`
  (`parent.UserConstructionScript`))