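; BP_Pot2_Breakable is a breakable pot Blueprint that plays a shatter sound and dissolves once broken.
; GetHit plays the sound at the impact point, then defers to the parent.
; The Chaos break event calls DissolveBroken with a pottery material and lifespan, then runs a timeline driving DissolveAmount on each DissolveMat material.
; That timeline update also calls parent GetHit at the actor's location for every material.
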(event `HitInterface.GetHit`
  (params (ImpactPoint :type "Vector Structure (by ref)") (Hitter :type "Actor Object Reference"))
  (`GameplayStatics.PlaySoundAtLocation` "/Game/Assets/Audio/MetaSounds/sfx_PotBreak.sfx_PotBreak" ImpactPoint (struct) 1.0 1.0 0.0 null null null null)
  (`parent.GetHit` ImpactPoint null))

(event `self.GeometryCollection.OnChaosBreakEvent`
  (params (BreakEvent :type "ChaosBreakEvent Structure (by ref)"))
  (`self.DissolveBroken` 5.0 (`|MakeArray` "/Game/Destructibles/Materials/MI_Pottery_01.MI_Pottery_01" :!type "MaterialInstance Object Reference"))
  (bind (_direction _newtrack_0) (`Timeline|Dissolve`)
    (:`Update`
      (for _array_element (`self.DissolveMat`)
        (`MaterialInstanceDynamic.SetScalarParameterValue` _array_element "DissolveAmount" _newtrack_0)
        (`parent.GetHit` (`self.K2_GetActorLocation`) null)))))

(fn `UserConstructionScript`
  (`parent.UserConstructionScript`))