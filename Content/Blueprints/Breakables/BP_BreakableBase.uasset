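; Base breakable actor built on a Chaos geometry collection and a capsule, with hit behavior inherited from its parent.
; On a Chaos break it sets a short lifespan, makes the capsule ignore all collision and calls the parent GetHit at the actor location.
; DissolveBroken similarly retires the actor and swaps in dynamic material instances from supplied materials, but its DissolveAmount parameter setter is unconnected.
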(event `self.GeometryCollection.OnChaosBreakEvent`
  (params (BreakEvent :type "ChaosBreakEvent Structure (by ref)"))
  (`self.SetLifeSpan` 5.0)
  (`PrimitiveComponent.SetCollisionResponseToAllChannels` (`self.Capsule`) "ECR_Ignore")
  (`parent.GetHit` (`self.K2_GetActorLocation`) null))

(fn `DissolveBroken`
  (params (LifeSpan :type "Float (double-precision)") (Material :type "Array of MaterialInstance Object Reference"))
  (`self.SetLifeSpan` LifeSpan)
  (`PrimitiveComponent.SetCollisionResponseToAllChannels` (`self.Capsule`) "ECR_Ignore")
  (for _array_element Material
    (bind _returnvalue (`PrimitiveComponent.CreateDynamicMaterialInstance` (`self.GeometryCollection`) 0 _array_element "None"))
    (`KismetArrayLibrary.Array_Add` (`self.DissolveMat`) _returnvalue))
  (for (_array_element_2 _array_index) (`self.DissolveMat`)
    (`PrimitiveComponent.SetMaterial` (`self.GeometryCollection`) _array_index _array_element_2)))

(fn `UserConstructionScript`)